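; VideoPlane is an actor that slides a plane into view and plays a video when a referenced listener's value goes over its limit.
; On that event it unbinds, opens a hardcoded media source and runs a timeline that lerps the plane between markers A and B.
; When the video ends, it resets the listener's progress, reverses the timeline and rebinds for the next trigger.
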(event Custom|Initiate
  (EventDispatchers|UnbindEventfromValueOverLimit (Variables|Default|GetListenerRef) (delegate Custom|Initiate))
  ;[0 0 0 1 11] Video Start and Transition logic
  (Media|MediaPlayer|OpenSource (Variables|Default|GetPlayer) "/Game/Videos/Are_You_Ready_-_Steam_Summer_Sale_2016.Are_You_Ready_-_Steam_Summer_Sale_2016")
  (bind _atdistance (Timeline|Timeline_0 PlayFromStart)
    (:Update
      (Transformation|SetWorldLocation (Variables|Default|GetPlane) (Math|Vector|Lerp(Vector) (Transformation|GetWorldLocation (Variables|Default|GetA)) (Transformation|GetWorldLocation (Variables|Default|GetB)) _atdistance) false false))))

(event Custom|VideoFinished
  (Variables|/Game/Blueprints/Button.Button_C|Setf_ProgressValue (Variables|Default|GetListenerRef) 0.0)
  (Components|Timeline|ReversefromEnd (Variables|Default|GetTimeline_0))
  (CallFunction|Rebind))

(event Custom|Rebind
  (EventDispatchers|BindEventtoValueOverLimit (Variables|Default|GetListenerRef) (delegate Custom|Initiate)))

(event EventBeginPlay
  (Media|MediaPlayer|BindEventtoOnEndReached (Variables|Default|GetPlayer) (delegate Custom|VideoFinished))
  (EventDispatchers|BindEventtoValueOverLimit (Variables|Default|GetListenerRef) (delegate Custom|Initiate)))

(event Collision|EventActorBeginOverlap
  (params (OtherActor :type Actor%20Object%20Reference)))

(event EventTick
  (params (DeltaSeconds :type Float%20%28single-precision%29)))

(fn ConstructionScript)