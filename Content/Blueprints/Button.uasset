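; Pressable button actor that fills a progress value on repeated presses and fires ValueOverLimit once it reaches full.
; Capsule overlap triggers a press, which adds progress, plays a sound and briefly squashes and recolors the mesh.
; Tick uses a Delay to drain progress periodically while it is within range.
; On BeginPlay it passes itself to its Button_ProgressBar widget as a reference.
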(event OnComponentBeginOverlap(Capsule)
  (params (OverlappedComponent :type Primitive%20Component%20Object%20Reference) (OtherActor :type Actor%20Object%20Reference) (OtherComp :type Primitive%20Component%20Object%20Reference) (OtherBodyIndex :type Integer) (bFromSweep :type Boolean) (SweepResult :type Hit%20Result%20Structure%20%28by%20ref%29))
  (CallFunction|ButtonPressed))

(event Custom|Button_Pressed
  (bind _button (Variables|Default|GetButton))
  (bind _button_2 (Variables|Default|GetButton))
  (if (not (>= (Variables|Default|Getf_ProgressValue) 1.0))
    (CallFunction|ProgressValueChange (Variables|Default|GetIncrementValue))
    (Audio|PlaySoundatLocation "/Game/Sounds/SoundButton.SoundButton" (Transformation|GetActorLocation) "0, 0, 0" 0.5 1.0 0.0 0 0 0)
    ;[0.005208 0.005208 0.005208 1 11] change mat and scale for press feedback
    (Transformation|SetWorldScale3D _button_2 "0.500000,0.500000,1.700000")
    (Rendering|Material|SetMaterial _button_2 0 "/Game/Material/Green.Green")
    (Utilities|FlowControl|Delay 0.2)
    (Transformation|SetWorldScale3D _button "0.500000,0.500000,2.000000")
    (Rendering|Material|SetMaterial _button 0 "/Game/VirtualReality/Materials/M_BaseMaterial.M_BaseMaterial")))

(event EventBeginPlay
  ;[0 0 0 1 11] Set ref in widget
  (Variables|/Game/Widget/Button_ProgressBar.Button_ProgressBar_C|SetReference_Actor (.AsButton%20Progress%20Bar (Utilities|Casting|CastToButton_ProgressBar (UserInterface|GetUserWidgetObject (Variables|Default|GetWidget)))) self))

(event Collision|EventActorBeginOverlap
  (params (OtherActor :type Actor%20Object%20Reference)))

(event EventTick
  (params (DeltaSeconds :type Float%20%28single-precision%29))
  ;[0 0 0 1 11] decrease per timer
  (if (Math|Float|InRange(Float) (Variables|Default|Getf_ProgressValue) 0.0 1.0 false false)
    (Utilities|FlowControl|Delay (Variables|Default|GetDecrementSpeed))
    (CallFunction|ProgressValueChange (Variables|Default|GetDecrementValue))))

(fn ConstructionScript)

(fn ProgressValueChange
  (params (ChangeBy :type Float%20%28single-precision%29))
  (bind _output_get (Variables|Default|Setf_ProgressValue (+ (Variables|Default|Getf_ProgressValue) ChangeBy)))
  (if (>= _output_get 1.0)
    (Default|CallValueOverLimit)))